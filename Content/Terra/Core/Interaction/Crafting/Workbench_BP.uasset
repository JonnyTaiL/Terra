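; Workbench Blueprint that serves as an interactable crafting station.
; Its Interactwith event stores the interacting player reference and toggles the crafting view through that player's TerraHUD.
; An unconnected graph fragment would rotate a visible component toward the player vessel's camera using look-at pitch and yaw, but it never runs.
; BeginPlay, Tick and the construction script add no logic of their own.
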(event `self.ReceiveBeginPlay`)

(event `/Game/Terra/Core/Interfaces/IPlayerInteract.InteractWith`
  (params (PlayerRef :type "/Game/Terra/Characters/TerraCharacterBase_BP Object Reference"))
  (bind _output_get (set `self.Player Ref` PlayerRef))
  (`/Game/Terra/Core/Interaction/UI/Terra_HUD.ToggleCraft` (`/Game/Terra/Characters/TerraCharacterBase_BP.TerraHUD` _output_get)))

(event `self.ReceiveTick`
  (params (DeltaSeconds :type "Float (single-precision)")))

(fn `UserConstructionScript`
  (`parent.UserConstructionScript`))