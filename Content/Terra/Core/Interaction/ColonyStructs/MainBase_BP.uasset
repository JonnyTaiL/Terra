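; MainBase_BP is the colony's main base structure, providing an oxygen zone around itself.
; A Size value, applied at construction, drives both the Niagara circle and the overlap sphere radius.
; While Enabled, the sphere sends expose-to-oxygen messages to entering actors, and remove messages on exit.
; Interaction and level-up events are empty; the three-tier resource upgrade logic and its widget are disconnected.
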(event `SetSize`
  (params (Size :type "Float (double-precision)" :default 0.02))
  (set `self.Size` Size)
  (`NiagaraComponent.SetVariableFloat` (`self.Niagara`) "CircleSize" (`self.Size`))
  (`SphereComponent.SetSphereRadius` (`self.Sphere`) (* 130.0 (* (`self.Size`) 100.0)) true))

(event `self.Sphere.OnComponentBeginOverlap`
  (params (OverlappedComponent :type "PrimitiveComponent Object Reference") (OtherActor :type "Actor Object Reference") (OtherComp :type "PrimitiveComponent Object Reference") (OtherBodyIndex :type Integer) (bFromSweep :type Boolean) (SweepResult :type "HitResult Structure (by ref)"))
  (if (`self.bEnabled`)
    (message `/Game/Terra/Core/Interfaces/IOxygenReaction.ExposeToOxygen` OtherActor)))

(event `self.ReceiveBeginPlay`)

(event `self.SphereUI.OnComponentBeginOverlap`
  (params (OverlappedComponent :type "PrimitiveComponent Object Reference") (OtherActor :type "Actor Object Reference") (OtherComp :type "PrimitiveComponent Object Reference") (OtherBodyIndex :type Integer) (bFromSweep :type Boolean) (SweepResult :type "HitResult Structure (by ref)")))

(event `self.Sphere.OnComponentEndOverlap`
  (params (OverlappedComponent :type "PrimitiveComponent Object Reference") (OtherActor :type "Actor Object Reference") (OtherComp :type "PrimitiveComponent Object Reference") (OtherBodyIndex :type Integer))
  (message `/Game/Terra/Core/Interfaces/IOxygenReaction.RemoveFromOxygen` OtherActor))

(event `/Game/Terra/Core/Interfaces/IPlayerInteract.LookAt`
  (params (PlayerRef :type "/Game/Terra/Characters/TerraCharacterBase_BP Object Reference")))

(event `/Game/Terra/Core/Interfaces/IPlayerInteract.LoseFocus`
  (params (PlayerRef :type "/Game/Terra/Characters/TerraCharacterBase_BP Object Reference")))

(event `/Game/Terra/Core/Interfaces/IPlayerInteract.InteractWith`
  (params (PlayerRef :type "/Game/Terra/Characters/TerraCharacterBase_BP Object Reference")))

(event `LevelUP`)

(fn `UserConstructionScript`
  (`self.SetSize` (`self.Size`))
  (`parent.UserConstructionScript`))