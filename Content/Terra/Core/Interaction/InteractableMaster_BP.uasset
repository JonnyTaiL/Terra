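; InteractableMaster_BP is the master interactable actor, handling player look-at focus and interaction with a prompt widget.
; Lookat stores itself as the player's LookAtActor, tells the previous target to lose focus, and shows its Widget; losing focus hides it.
; Interactwith only prints a debug message naming player and object.
; Disconnected leftover nodes hold an array-based focus and item pickup approach that never runs.
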(event `Local_LoseFocus`
  (`SceneComponent.SetVisibility` (`self.Widget`) false false :!label _label)
  (`KismetSystemLibrary.PrintString` "Bruh"))

(event `/Game/Terra/Core/Interfaces/IPlayerInteract.LoseFocus`
  (params (PlayerRef :type "/Game/Terra/Characters/TerraCharacterBase_BP Object Reference"))
  (goto _label))

(event `/Game/Terra/Core/Interfaces/IPlayerInteract.LookAt`
  (params (PlayerRef :type "/Game/Terra/Characters/TerraCharacterBase_BP Object Reference"))
  (bind _lookatactor (`/Game/Terra/Characters/TerraCharacterBase_BP.LookAtActor` PlayerRef))
  (if (!= _lookatactor self)
    (`/Engine/EditorBlueprintResources/StandardMacros.IsValid` _lookatactor
      (:`Is Valid`
        (message `/Game/Terra/Core/Interfaces/IPlayerInteract.LoseFocus` _lookatactor PlayerRef))
      (:`Is Not Valid`
        _))
    (set `/Game/Terra/Characters/TerraCharacterBase_BP.LookAtActor` self PlayerRef)
    (`SceneComponent.SetVisibility` (`self.Widget`) true false)))

(event `/Game/Terra/Core/Interfaces/IPlayerInteract.InteractWith`
  (params (PlayerRef :type "/Game/Terra/Characters/TerraCharacterBase_BP Object Reference"))
  (`KismetSystemLibrary.PrintString` (`KismetTextLibrary.Conv_TextToString` (`|FormatText` "Player {player} Interacted With Object - {object}" PlayerRef (`/Game/Terra/Characters/TerraCharacterBase_BP.LookAtActor` PlayerRef)))))

(fn `UserConstructionScript`)