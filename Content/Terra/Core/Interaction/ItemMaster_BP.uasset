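; ItemMaster_BP is an item Blueprint, apparently a base for interactable items, that handles a player's look-at focus.
; Lookat makes the item the player's LookAtActor, first sending LoseFocusMessage to any valid previous target.
; LoseFocus and CustomEvent are empty.
; Disconnected leftover nodes hold unused logic for widget visibility, an array of looked-at actors, interaction debug prints and destroying the item.
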(event `CustomEvent`)

(event `/Game/Terra/Core/Interfaces/IPlayerInteract.LoseFocus`
  (params (PlayerRef :type "/Game/Terra/Characters/TerraCharacterBase_BP Object Reference")))

(event `/Game/Terra/Core/Interfaces/IPlayerInteract.LookAt`
  (params (PlayerRef :type "/Game/Terra/Characters/TerraCharacterBase_BP Object Reference"))
  (bind _lookatactor (`/Game/Terra/Characters/TerraCharacterBase_BP.LookAtActor` PlayerRef))
  (if (!= _lookatactor self)
    (`/Engine/EditorBlueprintResources/StandardMacros.IsValid` _lookatactor
      (:`Is Valid`
        (message `/Game/Terra/Core/Interfaces/IPlayerInteract.LoseFocus` _lookatactor PlayerRef))
      (:`Is Not Valid`
        _))
    (set `/Game/Terra/Characters/TerraCharacterBase_BP.LookAtActor` self PlayerRef)))

(fn `UserConstructionScript`
  (`parent.UserConstructionScript`))