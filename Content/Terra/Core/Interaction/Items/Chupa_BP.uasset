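; Chupa_BP is an interaction item that transforms into a Chapa_BP when exposed to oxygen.
; ExposetoOxygen sets the UnderOxygen flag, waits five seconds, then spawns Chapa_BP at its transform and destroys itself if the flag still holds.
; RemovefromOxygen clears the flag to cancel a pending transformation, and both events print debug messages.
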(event `/Game/Terra/Core/Interfaces/IOxygenReaction.ExposeToOxygen`
  (`KismetSystemLibrary.PrintString` "Chupa Is Transforming!!!!" true true (struct :`R` 1.0 :`B` 0.055182 :`A` 1.0) 5.0)
  (set `self.bUnderOxygen` true)
  (`KismetSystemLibrary.Delay` 5.0)
  (if (`self.bUnderOxygen`)
    (`|SpawnActorFromClass` "/Game/Terra/Core/Interaction/Items/Chapa_BP.Chapa_BP_C" (`self.GetTransform`) "Undefined" "MultiplyWithRoot" null null)
    (`self.K2_DestroyActor`)))

(event `/Game/Terra/Core/Interfaces/IOxygenReaction.RemoveFromOxygen`
  (`KismetSystemLibrary.PrintString` "Chupa Is Not Tranforming" true true (struct :`R` 1.0 :`B` 0.055182 :`A` 1.0) 5.0)
  (set `self.bUnderOxygen` false)
  (`KismetSystemLibrary.Delay` 5.0))

(fn `UserConstructionScript`
  (`parent.UserConstructionScript`))