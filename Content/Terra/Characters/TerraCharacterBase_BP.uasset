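; Base player character for Terra, shown as a Fish or Rabbit flipbook sprite chosen by PlayerIndex.
; BeginPlay sets up input, HUD and the shared OxygenVessel, whose camera rotation index remaps movement to world axes.
; Sphere overlaps drive look-at messages; Interact messages the focused actor and overlapping MainBase, then refreshes inventory HUD.
; A source counter feeds oxygen gain and loss to PlayerStatsBP, alongside debug keys and on-screen prints.
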(event OnComponentBeginOverlap(Sphere)
  (params (OverlappedComponent :type Primitive%20Component%20Object%20Reference) (OtherActor :type Actor%20Object%20Reference) (OtherComp :type Primitive%20Component%20Object%20Reference) (OtherBodyIndex :type Integer) (bFromSweep :type Boolean) (SweepResult :type Hit%20Result%20Structure%20%28by%20ref%29))
  (Class|IPlayerInteract|Lookat(Message) OtherActor self))

(event OnComponentEndOverlap(Sphere)
  (params (OverlappedComponent :type Primitive%20Component%20Object%20Reference) (OtherActor :type Actor%20Object%20Reference) (OtherComp :type Primitive%20Component%20Object%20Reference) (OtherBodyIndex :type Integer))
  (Class|IPlayerInteract|LoseFocus(Message) (Variables|Default|GetLookAtActor) self)
  (Variables|Default|SetLookAtActor 0))

(event Custom|SetView
  (params (Vessel :type Actor%20Object%20Reference))
  ;[0.1042 0.1042 0.1042] Initial Setup
  (bind _asterra_controller_bp (Utilities|Casting|CastToTerraController_BP (Pawn|GetController)))
  (Game|Player|SetViewTargetwithBlend _asterra_controller_bp Vessel 1.0 "VTBlend_Linear" 0.0 false))

(event Input|EnhancedActionEvents|EnhancedInputActionIA_Move
  (params (ActionValue :type Vector%202D%20Structure) (ElapsedSeconds :type Float%20%28double-precision%29) (TriggeredSeconds :type Float%20%28double-precision%29) (InputAction :type Input%20Action%20Object%20Reference :default "/Game/Terra/Characters/Inputs/IA_Move.IA_Move"))
  (Pawn|Input|AddMovementInput (Utilities|Select :Index (Variables|/Game/Terra/Characters/OxygenVessel_BP.OxygenVessel_BP_C|GetCameraRotIndex (Variables|Default|GetVesselRef)) :Option%200 "0.000000,1.000000,0.000000" :Option%201 "-1.000000,0.000000,0.000000" :Option%202 "0.000000,-1.000000,0.000000" :Option%203 "1.000000,0.000000,0.000000") (.x ActionValue) false)
  (Pawn|Input|AddMovementInput (Utilities|Select :Index (Variables|/Game/Terra/Characters/OxygenVessel_BP.OxygenVessel_BP_C|GetCameraRotIndex (Variables|Default|GetVesselRef)) :Option%200 "1.000000,0.000000,0.000000" :Option%201 "0.000000,1.000000,0.000000" :Option%202 "-1.000000,0.000000,0.000000" :Option%203 "0.000000,-1.000000,0.000000") (.y ActionValue) false))

(event Input|EnhancedActionEvents|EnhancedInputActionIA_Interact
  (params (ActionValue :type Boolean) (ElapsedSeconds :type Float%20%28double-precision%29) (TriggeredSeconds :type Float%20%28double-precision%29) (InputAction :type Input%20Action%20Object%20Reference :default "/Game/Terra/Characters/Inputs/IA_Interact.IA_Interact"))
  (:Started
    (Utilities|FlowControl|Sequence
      (:then_0
        (bind _lookatactor (Variables|Default|GetLookAtActor)
          (:then
            (Class|IPlayerInteract|Interactwith(Message) _lookatactor self)
            (bind _asterra_controller_bp (Utilities|Casting|CastToTerraController_BP (Game|GetPlayerController (Variables|Default|GetPlayerIndex))))
            (Default|UpdateInventoryHUD _asterra_controller_bp)
            (Class|IPlayerInteract|Lookat(Message) (Utilities|Array|Get(acopy) (Collision|GetOverlappingActors (Variables|Default|GetSphere) "/Game/Terra/Core/Interaction/InteractableMaster_BP.InteractableMaster_BP_C" :!class /Script/Engine.PrimitiveComponent)) self))
          (:else)))
      (:then_1
        (for _array_element (Collision|GetOverlappingActors "/Game/Terra/Core/Interaction/ColonyStructs/MainBase_BP.MainBase_BP_C" :!class /Script/Engine.Actor)
          (Class|IPlayerInteract|Interactwith(Message) _array_element self)
          (bind _asterra_controller_bp_2 (Utilities|Casting|CastToTerraController_BP (Game|GetPlayerController (Variables|Default|GetPlayerIndex))))
          (Default|UpdateInventoryHUD _asterra_controller_bp_2))))))

(event Input|EnhancedActionEvents|EnhancedInputActionIA_Inventory
  (params (ActionValue :type Boolean) (ElapsedSeconds :type Float%20%28double-precision%29) (TriggeredSeconds :type Float%20%28double-precision%29) (InputAction :type Input%20Action%20Object%20Reference :default "/Game/Terra/Characters/Inputs/IA_Inventory.IA_Inventory"))
  (:Started
    (Default|DEBUGPrintContents (Variables|Default|GetInventorySystem_BP))))

(event EventBeginPlay
  (Utilities|FlowControl|Sequence
    (:then_0
      ;[0.1042 0.1042 0.1042] Initial Setup
      (Utilities|FlowControl|Delay 0.2)
      (CallFunction|InitializeIMC)
      (bind _returnvalue (Actor|GetActorOfClass "/Game/Terra/Characters/OxygenVessel_BP.OxygenVessel_BP_C"))
      (bind _output_get (Variables|Default|SetVesselRef _returnvalue))
      (Default|Initialize _output_get)
      (bind _asterra_hud (Utilities|Casting|CastToTerra_HUD (HUD|GetHUD (Game|GetPlayerController 0))))
      (bind _output_get_2 (Variables|Default|SetTerraHUD _asterra_hud))
      (Default|Initialize _output_get_2)
      (Sprite|SetFlipbook (Variables|Default|GetPaperFlipbook) (Utilities|Select :Index (Variables|Default|GetPlayerIndex) :Option%200 "/Game/Terra/Characters/Sprites/Fish/Idle/Front/Fish_Idle_Front.Fish_Idle_Front" :Option%201 "/Game/Terra/Characters/Sprites/Rabbit/Idle/Front/Rabbit_Idle_Front.Rabbit_Idle_Front")))))

(event EventExposetoOxygen
  (Default|OnGetOxygenSource (Variables|Default|GetPlayerStats_BP))
  (Math|Integer|IncrementInt (Variables|Default|GetOxygenSources)))

(event EventRemovefromOxygen
  (bind _result (Math|Integer|DecrementInt (Variables|Default|GetOxygenSources))
    (:%20%20
      (if (<= _result 0)
        (Default|OnLoseOxygenSource (Variables|Default|GetPlayerStats_BP))))))

(event EventTick
  (params (DeltaSeconds :type Float%20%28single-precision%29))
  (Development|PrintString (Utilities|GetDisplayName (Variables|Default|GetLookAtActor)) true true "(R=0.000000,G=0.660000,B=1.000000,A=1.000000)" DeltaSeconds)
  (Development|PrintString (Utilities|String|Append (Utilities|GetDisplayName self) " - " (Utilities|String|ToString(Float) (Variables|/Game/Terra/Characters/PlayerStats_BP.PlayerStats_BP_C|GetOxygen (Variables|Default|GetPlayerStats_BP)))) true true "(R=0.000000,G=0.660000,B=1.000000,A=1.000000)" DeltaSeconds))

(event Input|KeyboardEvents|DebugKey8
  (params (Key :type Key%20Structure :default "None") (ActionValue :type Input%20Action%20Value%20Structure))
  (:Pressed
    (bind _returnvalue (Actor|GetActorOfClass "/Game/Terra/Core/Interaction/ColonyStructs/MainBase_BP.MainBase_BP_C"))
    (Variables|/Game/Terra/Core/Interaction/ColonyStructs/MainBase_BP.MainBase_BP_C|SetSize _returnvalue 0.4)
    (Default|SetSize _returnvalue 0.02)))

(event Input|KeyboardEvents|DebugKey4
  (params (Key :type Key%20Structure :default "None") (ActionValue :type Input%20Action%20Value%20Structure))
  (:Pressed
    (Default|TakeDamage (Variables|Default|GetPlayerStats_BP) 25.0)))

(event Input|KeyboardEvents|DebugKey2
  (params (Key :type Key%20Structure :default "None") (ActionValue :type Input%20Action%20Value%20Structure))
  (:Pressed
    (Default|ToggleCraft (Variables|Default|GetTerraHUD))))

(event Input|KeyboardEvents|PageUp
  (params (Key :type Key%20Structure :default "None"))
  (:Pressed
    (bind _vesselref (Variables|Default|GetVesselRef)
      (:then
        (Variables|/Script/Engine.SpringArmComponent|SetTargetArmLength (Variables|/Game/Terra/Characters/OxygenVessel_BP.OxygenVessel_BP_C|GetSpringArm _vesselref) (+ (Variables|/Script/Engine.SpringArmComponent|GetTargetArmLength (Variables|/Game/Terra/Characters/OxygenVessel_BP.OxygenVessel_BP_C|GetSpringArm _vesselref)) 5e+02)))
      (:else))))

(event Input|KeyboardEvents|PageDown
  (params (Key :type Key%20Structure :default "None"))
  (:Pressed
    (bind _vesselref (Variables|Default|GetVesselRef)
      (:then
        (Variables|/Script/Engine.SpringArmComponent|SetTargetArmLength (Variables|/Game/Terra/Characters/OxygenVessel_BP.OxygenVessel_BP_C|GetSpringArm _vesselref) (- (Variables|/Script/Engine.SpringArmComponent|GetTargetArmLength (Variables|/Game/Terra/Characters/OxygenVessel_BP.OxygenVessel_BP_C|GetSpringArm _vesselref)) 5e+02)))
      (:else))))

(event Input|MouseEvents|MiddleMouseButton
  (params (Key :type Key%20Structure :default "None"))
  (:Pressed
    (Default|RotateRight (Variables|Default|GetVesselRef))))

(fn ConstructionScript)

(fn InitializeIMC
  (bind _asterra_controller_bp (Utilities|Casting|CastToTerraController_BP (Class|GameplayStatics|GetPlayerControllerfromID (Variables|Default|GetPlayerIndex))))
  (Input|AddMappingContext (PlayerController|LocalPlayerSubsystems|GetEnhancedInputLocalPlayerSubsystem _asterra_controller_bp) "/Game/Terra/Characters/Inputs/IMC_Default.IMC_Default" 0 "(bIgnoreAllPressedKeysUntilRelease=True,bForceImmediately=False,bNotifyUserSettings=False)"))