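; OxygenVessel_BP is a shared view target for Terra characters that tracks the midpoint between them.
; Initialize gathers all TerraCharacterBase_BP actors into PlayerArray and passes itself to each through SetView.
; Each Tick, GetPlayersMedian sums valid character locations, halves the total (assuming two players) and draws a debug sphere there.
; The vessel itself never moves, and no oxygen logic is present.
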(event `self.ReceiveTick`
  (params (DeltaSeconds :type "Float (single-precision)"))
  (`self.GetPlayersMedian`))

(event `Initialize`
  (bind _outactors (`GameplayStatics.GetAllActorsOfClass` "/Game/Terra/Characters/TerraCharacterBase_BP.TerraCharacterBase_BP_C"))
  (bind _output_get (set `self.PlayerArray` _outactors))
  (for (_array_element _array_index) _output_get
    (set `self.Index` _array_index)
    (`/Game/Terra/Characters/TerraCharacterBase_BP.SetView` _array_element self)))

(fn `GetPlayersMedian`
  (returns (Median :type "Vector Structure"))
  (locals (Local_Pos :type "Array of Vector Structure") (Local_TempVector :type "Vector Structure"))
  (for _array_element (`self.PlayerArray`)
    (`/Engine/EditorBlueprintResources/StandardMacros.IsValid` _array_element
      (:`Is Valid`
        (set `local.Local_TempVector` (+ (`self.K2_GetActorLocation` _array_element) (`local.Local_TempVector`))))))
  (bind _output_get (set `local.Local_TempVector` (/ (`local.Local_TempVector`) 2.0)))
  (`KismetSystemLibrary.DrawDebugSphere` _output_get 50.0)
  (return _output_get))

(fn `UserConstructionScript`)