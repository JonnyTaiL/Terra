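; Player controller for Terra that relays inventory refresh requests to the HUD.
; UpdateInventoryHUD casts the current HUD to Terra_HUD and calls Update on its inventory panel widget.
; InitUI is an empty event; a disconnected graph that would set game-only input and create the core and inventory panel widgets, passing all TerraCharacterBase_BP actors to the panel, never runs.
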(event `InitUI`)

(fn `UpdateInventoryHUD`
  (bind _asterra_hud (cast `/Game/Terra/Core/Interaction/UI/Terra_HUD` (`self.GetHUD`)))
  (`/Game/Terra/Core/Interaction/UI/WB_InventoryPanel.Update` (`/Game/Terra/Core/Interaction/UI/Terra_HUD.WB_InventoryPanel_HUD` _asterra_hud)))

(fn `UserConstructionScript`)