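; Base enemy pawn with flipbook animation that chases and bites the player character.
; Sphere overlap locks the first TerraCharacterBase_BP as target, and Tick issues AIMoveTo while switching idle/walk flipbooks by speed.
; AttackSphere overlap runs a looping timer that applies damage and plays the bite until the target leaves.
; Lethal damage plays death, spawns Chupa_BP, then destroys the actor; Type only sets the construction-time flipbook, which Tick overrides with Monster animations.
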(event `self.ReceiveAnyDamage`
  (params (Damage :type "Float (single-precision)") (DamageType :type "DamageType Object Reference") (InstigatedBy :type "Controller Object Reference") (DamageCauser :type "Actor Object Reference"))
  (bind _flipbook (`self.Flipbook`))
  (bind _returnvalue (- (`self.Health`) Damage))
  (if (<= _returnvalue 0.0)
    (set `self.bDead` true)
    (`PaperFlipbookComponent.SetFlipbook` _flipbook "/Game/Sakura/Front/Sprites_Monster/Anim/Flip_Monster_Die.Flip_Monster_Die")
    (`KismetSystemLibrary.K2_ClearAndInvalidateTimerHandle` (`self.Handle`))
    (`MovementComponent.StopMovementImmediately` (`self.CharacterMovement`))
    (`KismetSystemLibrary.Delay` 1.0)
    (`PaperFlipbookComponent.Stop` _flipbook)
    (`|SpawnActorFromClass` "/Game/Terra/Core/Interaction/Items/Chupa_BP.Chupa_BP_C" (`KismetMathLibrary.Conv_VectorToTransform` (`self.K2_GetActorLocation`)) "Undefined" "MultiplyWithRoot" null null)
    (`KismetSystemLibrary.Delay` 5.0)
    (`self.K2_DestroyActor`)
    (else
      (set `self.Health` _returnvalue))))

(event `self.ReceiveTick`
  (params (DeltaSeconds :type "Float (single-precision)"))
  (if (not (`self.bDead`))
    (set `self.Speed` (`KismetMathLibrary.VSize` (`self.GetVelocity`)))
    (`|ExecutionSequence`
      (:`then_0`
        (bind _enemyref (`self.EnemyRef`)
          (:`then`
            (`|AIMoveTo` self (0.0 0.0 0.0) _enemyref 20.0))
          (:`else`
            (`PaperFlipbookComponent.SetFlipbook` (`self.Flipbook`) "/Game/Sakura/Front/Sprites_Monster/Anim/Flip_Monster_Idle.Flip_Monster_Idle"))))
      (:`then_1`
        (if (not (`self.Attack?`))
          (if (> (`self.Speed`) 10.0)
            (`PaperFlipbookComponent.SetFlipbook` (`self.Flipbook`) "/Game/Sakura/Front/Sprites_Monster/Anim/Flip_Monster_Walk_Left.Flip_Monster_Walk_Left")
            (else
              (`PaperFlipbookComponent.SetFlipbook` (`self.Flipbook`) "/Game/Sakura/Front/Sprites_Monster/Anim/Flip_Monster_Idle.Flip_Monster_Idle"))))))))

(event `self.Sphere.OnComponentBeginOverlap`
  (params (OverlappedComponent :type "PrimitiveComponent Object Reference") (OtherActor :type "Actor Object Reference") (OtherComp :type "PrimitiveComponent Object Reference") (OtherBodyIndex :type Integer) (bFromSweep :type Boolean) (SweepResult :type "HitResult Structure (by ref)"))
  (bind _asterra_character_base_bp (cast `/Game/Terra/Characters/TerraCharacterBase_BP` OtherActor))
  (`self.EnemyRef`
    (:`then`)
    (:`else`
      (set `self.EnemyRef` _asterra_character_base_bp))))

(event `self.AttackSphere.OnComponentBeginOverlap`
  (params (OverlappedComponent :type "PrimitiveComponent Object Reference") (OtherActor :type "Actor Object Reference") (OtherComp :type "PrimitiveComponent Object Reference") (OtherBodyIndex :type Integer) (bFromSweep :type Boolean) (SweepResult :type "HitResult Structure (by ref)"))
  (if (== OtherActor (`self.EnemyRef`))
    (bind _returnvalue (`KismetSystemLibrary.K2_SetTimerDelegate` (delegate `Attack`) 2.0 true))
    (set `self.Handle` _returnvalue)))

(event `Attack`
  (`KismetSystemLibrary.PrintString` "AAttack")
  (`GameplayStatics.ApplyDamage` (`self.EnemyRef`) 10.0)
  (set `self.Attack?` true)
  (`PaperFlipbookComponent.SetFlipbook` (`self.Flipbook`) "/Game/Sakura/Front/Sprites_Monster/Anim/Flip_Monster_Bite.Flip_Monster_Bite")
  (`KismetSystemLibrary.Delay` 1.0)
  (set `self.Attack?` false))

(event `self.AttackSphere.OnComponentEndOverlap`
  (params (OverlappedComponent :type "PrimitiveComponent Object Reference") (OtherActor :type "Actor Object Reference") (OtherComp :type "PrimitiveComponent Object Reference") (OtherBodyIndex :type Integer))
  (if (== OtherActor (`self.EnemyRef`))
    (`KismetSystemLibrary.K2_ClearAndInvalidateTimerHandle` (`self.Handle`))))

(fn `UserConstructionScript`
  (switch `int` (`self.Type`)
    (:`0`
      (`PaperFlipbookComponent.SetFlipbook` (`self.Flipbook`) "/Game/Sakura/Front/Sprites_Monster/Anim/Flip_Monster_Idle.Flip_Monster_Idle"))
    (:`1`
      (`PaperFlipbookComponent.SetFlipbook` (`self.Flipbook`) "/Game/Sakura/Front/Sprites_Monster/Anim/Flip_Shmel_Fly.Flip_Shmel_Fly"))))